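; Base enemy Blueprint that uses the Gameplay Ability System and displays an attribute value on its Health text.
; On BeginPlay it grants the GA_Shoot ability to its ability system; nothing in this Blueprint activates it.
; The Health text is set from the attribute in the construction script and refreshed by polling every Tick.
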(event EventBeginPlay
  (GameplayAbilities|GiveAbility (Variables|Default|GetAbilitySystem) "/Game/GameplayAbilities/GA_Shoot.GA_Shoot_C" 0 -1))

(event EventTick
  (params (DeltaSeconds :type Float%20%28single-precision%29))
  (Rendering|Components|TextRender|SetText (Variables|Default|GetHealth) (Utilities|Text|ToText(Float) (.ReturnValue (Class|AbilitySystemComponent|GetGameplayAttributeValue (Variables|Default|GetAbilitySystem) "(AttributeName=\"Health\",Attribute=/Script/ParaTest.PTAttributeSet:Health,AttributeOwner=\"/Script/CoreUObject.Class'/Script/ParaTest.PTAttributeSet'\")")) "HalfToEven")))

(fn ConstructionScript
  (Rendering|Components|TextRender|SetText (Variables|Default|GetHealth) (Utilities|Text|ToText(Float) (.ReturnValue (Class|AbilitySystemComponent|GetGameplayAttributeValue (Variables|Default|GetAbilitySystem) "(AttributeName=\"Health\",Attribute=/Script/ParaTest.PTAttributeSet:Health,AttributeOwner=\"/Script/CoreUObject.Class'/Script/ParaTest.PTAttributeSet'\")")) "HalfToEven")))