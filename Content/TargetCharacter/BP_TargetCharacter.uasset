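; BP_TargetCharacter is a target character that displays a Gameplay Ability System attribute as text through its Health component.
; The construction script caches the mesh's first material as BaseMaterial and sets the initial text, and Tick refreshes that text from the AbilitySystem every frame.
; ChangeColor applies a given material to that mesh slot, or restores BaseMaterial when the given material is invalid.
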(event EventBeginPlay)

(event Collision|EventActorBeginOverlap
  (params (OtherActor :type Actor%20Object%20Reference)))

(event EventTick
  (params (DeltaSeconds :type Float%20%28single-precision%29))
  (Rendering|Components|TextRender|SetText (Variables|Default|GetHealth) (Utilities|Text|ToText(Float) (.ReturnValue (Class|AbilitySystemComponent|GetGameplayAttributeValue (Variables|Default|GetAbilitySystem) "(AttributeName=\"Health\",Attribute=/Script/ParaTest.PTAttributeSet:Health,AttributeOwner=\"/Script/CoreUObject.Class'/Script/ParaTest.PTAttributeSet'\")")) "HalfToEven")))

(fn ConstructionScript
  (Variables|Default|SetBaseMaterial (Rendering|Material|GetMaterial (Variables|Default|GetMeshComponent) 0))
  (Rendering|Components|TextRender|SetText (Variables|Default|GetHealth) (Utilities|Text|ToText(Float) (.ReturnValue (Class|AbilitySystemComponent|GetGameplayAttributeValue (Variables|Default|GetAbilitySystem) "(AttributeName=\"Health\",Attribute=/Script/ParaTest.PTAttributeSet:Health,AttributeOwner=\"/Script/CoreUObject.Class'/Script/ParaTest.PTAttributeSet'\")")) "HalfToEven")))

(fn ChangeColor
  (params (NewMaterial :type Material%20Interface%20Object%20Reference))
  (bind _meshcomponent (Variables|Default|GetMeshComponent))
  (Utilities|IsValid NewMaterial
    (:Is%20Valid
      (Rendering|Material|SetMaterial _meshcomponent 0 NewMaterial))
    (:Is%20Not%20Valid
      (Rendering|Material|SetMaterial _meshcomponent 0 (Variables|Default|GetBaseMaterial))))
  (return))